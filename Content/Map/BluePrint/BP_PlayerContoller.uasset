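; BP_PlayerContoller is a player controller that drives a pawn with a spring-arm camera on a map.
; BeginPlay adds the Enhanced Input mapping context, shows the main UI widget, and caches the pawn and starting control rotation.
; Input actions move the pawn along forward and right vectors, yaw it, and zoom by adjusting arm length within clamped limits.
; The jump action restores the starting rotation instead of jumping.
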(event Input|EnhancedActionEvents|EnhancedInputActionMoveInputAction
  (params (ActionValue :type Vector%202D%20Structure) (ElapsedSeconds :type Float%20%28double-precision%29) (TriggeredSeconds :type Float%20%28double-precision%29) (InputAction :type Input%20Action%20Object%20Reference :default "/Game/Map/Input/MoveInputAction.MoveInputAction"))
  (bind (_x _y) (Math|Vector2D|BreakVector2D ActionValue))
  (bind _returnvalue (Transformation|GetActorForwardVector))
  (bind _returnvalue_2 (Transformation|GetActorRightVector))
  (bind _pawncontr (Variables|Default|GetPawnContr))
  ;[0.15 0.15 0.15 0.5] 移动
  (Pawn|Input|AddMovementInput _pawncontr (Math|Vector|MakeVector (.x _returnvalue) (.y _returnvalue) 0.0) _x false)
  (Pawn|Input|AddMovementInput _pawncontr (Math|Vector|MakeVector (.x _returnvalue_2) (.y _returnvalue_2) 0.0) _y false))

(event Input|EnhancedActionEvents|EnhancedInputActionRotationInputAction
  (params (ActionValue :type Float%20%28double-precision%29) (ElapsedSeconds :type Float%20%28double-precision%29) (TriggeredSeconds :type Float%20%28double-precision%29) (InputAction :type Input%20Action%20Object%20Reference :default "/Game/Map/Input/RotationInputAction.RotationInputAction"))
  ;[0.15 0.15 0.15 0.5] 旋转
  (Pawn|Input|AddControllerYawInput (Variables|Default|GetPawnContr) ActionValue))

(event Input|EnhancedActionEvents|EnhancedInputActionJumpInputAction
  (params (ActionValue :type Boolean) (ElapsedSeconds :type Float%20%28double-precision%29) (TriggeredSeconds :type Float%20%28double-precision%29) (InputAction :type Input%20Action%20Object%20Reference :default "/Game/Map/Input/JumpInputAction.JumpInputAction"))
  ;[0.15 0.15 0.15 0.5] 恢复默认旋转
  (Pawn|SetControlRotation (Variables|Default|GetDefaultRotation)))

(event Input|EnhancedActionEvents|EnhancedInputActionUporDownInputAction
  (params (ActionValue :type Float%20%28double-precision%29) (ElapsedSeconds :type Float%20%28double-precision%29) (TriggeredSeconds :type Float%20%28double-precision%29) (InputAction :type Input%20Action%20Object%20Reference :default "/Game/Map/Input/UporDownInputAction.UporDownInputAction"))
  (bind _pawncontr (Variables|Default|GetPawnContr))
  (bind _returnvalue (Actor|GetComponentbyClass _pawncontr "/Script/Engine.SpringArmComponent"))
  (Variables|/Script/Engine.SpringArmComponent|SetTargetArmLength _returnvalue (Math|Float|Clamp(Float) (+ (Variables|/Script/Engine.SpringArmComponent|GetTargetArmLength _returnvalue) (* ActionValue 1e+01)) 5e+02 1.5e+03)))

(event EventBeginPlay
  (bind _returnvalue (Game|Player|GetPlayerPawn 0))
  (Input|AddMappingContext (PlayerController|LocalPlayerSubsystems|GetEnhancedInputLocalPlayerSubsystem) "/Game/Map/Input/Input_MappingContext.Input_MappingContext" 0 "(bIgnoreAllPressedKeysUntilRelease=True,bForceImmediately=False,bNotifyUserSettings=False)")
  (bind _returnvalue_2 (UserInterface|CreateWidget "/Game/Map/widget/BP_MianUserWidget.BP_MianUserWidget_C"))
  (UserInterface|Viewport|AddtoViewport _returnvalue_2 0)
  (Utilities|IsValid _returnvalue
    (:Is%20Valid
      (Variables|Default|SetPawnContr _returnvalue)
      (Variables|Default|SetDefaultRotation (Pawn|GetControlRotation :!class /Script/Engine.Controller)))))

(fn ConstructionScript)