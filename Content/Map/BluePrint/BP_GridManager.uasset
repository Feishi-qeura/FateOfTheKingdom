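; BP_GridManager is a map Blueprint that generates a square grid of mesh instances and places wall instances on selected cells.
; On BeginPlay, FUBuildGrid fills a HierarchicalInstancedStaticMesh at fixed spacing, recording each index in GridIndex and the middle one in CenterPointLocation.
; It then copies the local transforms of cells listed in WallIndex, which is not populated here, into a separate InstancedStaticMesh.
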(event EventBeginPlay
  (CallFunction|FUBuildGrid 50 50 1e+02)
  (for _array_element (Variables|Default|GetWallIndex)
    (Components|InstancedStaticMesh|AddInstance (Variables|Default|GetInstancedStaticMesh) (Math|Transform|MakeTransform (.location (.OutInstanceTransform (Components|InstancedStaticMesh|GetInstanceTransform (Variables|Default|GetHierarchicalInstancedStaticMesh) _array_element false))) (.rotation (.OutInstanceTransform (Components|InstancedStaticMesh|GetInstanceTransform (Variables|Default|GetHierarchicalInstancedStaticMesh) _array_element false))) (.scale (.OutInstanceTransform (Components|InstancedStaticMesh|GetInstanceTransform (Variables|Default|GetHierarchicalInstancedStaticMesh) _array_element false)))) false)))

(event Collision|EventActorBeginOverlap
  (params (OtherActor :type Actor%20Object%20Reference)))

(event EventTick
  (params (DeltaSeconds :type Float%20%28single-precision%29)))

(fn ConstructionScript)

(fn FUBuildGrid
  (params (Grid.X :type Integer) (Grid.Y :type Integer) (Offset :type Float%20%28double-precision%29))
  (for _index (range 0 Grid.X)
    (for _index_2 (range 0 Grid.Y)
      (bind _returnvalue (Components|InstancedStaticMesh|AddInstance (Variables|Default|GetHierarchicalInstancedStaticMesh) (Math|Transform|MakeTransform (Math|Vector|MakeVector (* _index Offset) (* _index_2 Offset) 0.0) "0, 0, 0" "1.000000,1.000000,1.000000") true))
      (Utilities|Array|Add (Variables|Default|GetGridIndex) _returnvalue)
      (if (and (== (/ Grid.X 2) _index) (== (/ Grid.Y 2) _index_2))
        (Variables|Default|SetCenterPointLocation _returnvalue)))))