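; Dialogue manager that runs data-table-driven conversations through a dialogue box widget with an embedded option box.
; BeginPlay creates the widget; ActivateDialogue, ignored while it is on screen, assigns the DataTable to both boxes.
; A single ID shows a dialogue line and multiple IDs show options.
; ReturnDialogueIDs feeds following IDs into the same flow; an empty list removes the widget, signals completion and clears the table.
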(event Custom|ActivateDialogue
  (params (BeginID :type Array%20of%20Names) (DataTable :type Data%20Table%20Object%20Reference))
  (bind _dialogue (Variables|Default|GetDialogue))
  (if (not (UserInterface|Viewport|IsinViewport (Variables|Default|GetDialogue)))
    (Variables|Default|SetBegin%20ID BeginID)
    (CallFunction|SetDataTable DataTable)
    (if (Utilities|Array|IsNotEmpty (Variables|Default|GetBegin%20ID))
      (if (not (UserInterface|Viewport|IsinViewport (Variables|Default|GetDialogue)))
        (UserInterface|Viewport|AddtoViewport (Variables|Default|GetDialogue) 100))
      (if (<= (Utilities|Array|Length (Variables|Default|GetBegin%20ID)) 1)
        (Default|UpdateDialogueData _dialogue (Utilities|Array|Get(acopy) (Variables|Default|GetBegin%20ID)))
        (else
          (Default|UpdateOptionData _dialogue (Variables|Default|GetBegin%20ID))))
      (elif (not (not (UserInterface|Viewport|IsinViewport (Variables|Default|GetDialogue))))
        (Widget|RemovefromParent (Variables|Default|GetDialogue))
        (Default|CallDialogueCompleted)
        (CallFunction|SetDataTable)))))

(event EventBeginPlay
  (bind _returnvalue (Game|ConstructObjectfromClass "/Game/Project/Shadow/BaseSystem/DialogueSystem/Widget/WBP_DialogueBox.WBP_DialogueBox_C" (Game|GetGameMode)))
  (bind _output_get (Variables|Default|SetDialogue _returnvalue))
  (Variables|Default|SetWBP%20Dialogue%20Option%20Box (Variables|/Game/Project/Shadow/BaseSystem/DialogueSystem/Widget/WBP_DialogueBox.WBP_DialogueBox_C|GetWBP_DialogueOptionBox _output_get)))

(event EventReturnDialogueIDs
  (params (DialogueIDs :type Array%20of%20Names))
  (bind _dialogue (Variables|Default|GetDialogue))
  (Variables|Default|SetBegin%20ID DialogueIDs)
  (if (Utilities|Array|IsNotEmpty (Variables|Default|GetBegin%20ID))
    (if (not (UserInterface|Viewport|IsinViewport (Variables|Default|GetDialogue)))
      (UserInterface|Viewport|AddtoViewport (Variables|Default|GetDialogue) 100))
    (if (<= (Utilities|Array|Length (Variables|Default|GetBegin%20ID)) 1)
      (Default|UpdateDialogueData _dialogue (Utilities|Array|Get(acopy) (Variables|Default|GetBegin%20ID)))
      (else
        (Default|UpdateOptionData _dialogue (Variables|Default|GetBegin%20ID))))
    (elif (not (not (UserInterface|Viewport|IsinViewport (Variables|Default|GetDialogue))))
      (Widget|RemovefromParent (Variables|Default|GetDialogue))
      (Default|CallDialogueCompleted)
      (CallFunction|SetDataTable))))

(fn ConstructionScript)

(fn SetDataTable
  (params (DataTable :type Data%20Table%20Object%20Reference))
  (bind _dialogue (Variables|Default|GetDialogue))
  (bind _wbp_dialogue_option_box (Variables|Default|GetWBP%20Dialogue%20Option%20Box))
  (Utilities|IsValid _dialogue
    (:Is%20Valid
      (Variables|/Game/Project/Shadow/BaseSystem/DialogueSystem/Widget/WBP_DialogueBox.WBP_DialogueBox_C|SetData%20Table _dialogue DataTable)
      (Utilities|IsValid _wbp_dialogue_option_box
        (:Is%20Valid
          (Variables|/Game/Project/Shadow/BaseSystem/DialogueSystem/Widget/WBP_DialogueOptionBox.WBP_DialogueOptionBox_C|SetData%20Table _wbp_dialogue_option_box DataTable))))))