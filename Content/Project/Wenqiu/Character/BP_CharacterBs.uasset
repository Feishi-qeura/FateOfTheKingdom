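; BP_CharacterBs is a character Blueprint, apparently a base class, that initializes its attributes when play begins.
; BeginPlay calls FUInitializeAttribute, which passes BaseAttribute to CharacterAttributes and then sets the max HP attribute to a hardcoded value.
; It prints the base attribute's MaxHealth afterward as debug output, while overlap, Tick and the construction script are empty.
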(event EventBeginPlay
  (CallFunction|FUInitializeAttribute))

(event Collision|EventActorBeginOverlap
  (params (OtherActor :type Actor%20Object%20Reference)))

(event EventTick
  (params (DeltaSeconds :type Float%20%28single-precision%29)))

(fn ConstructionScript)

(fn FUInitializeAttribute
  (bind _characterattributes (Variables|Default|GetCharacterAttributes))
  (Class|AttributeComponent|SetBaseAttribute _characterattributes (Variables|Default|GetBaseAttribute))
  (Class|AttributeComponent|SetAttribute _characterattributes "MAXHP" 1.5e+02)
  (Development|PrintString (Utilities|String|ToString(Float) (.MaxHealth (Utilities|Struct|BreakBaseAttribute (Variables|/Script/FateOfTheKingdom.AttributeComponent|GetBaseAttribute (Variables|Default|GetCharacterAttributes)))))))