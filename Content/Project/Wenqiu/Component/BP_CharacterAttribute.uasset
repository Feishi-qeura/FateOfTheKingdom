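; Character attribute component that holds a character's runtime stats in a single RuntimeAttribute struct.
; Separate initializers fill its base and combat attributes, faction and action bar avatar, with the enemy version also setting enemy type and occupation.
; Accessor functions expose the avatar, Speed and CurrentAV, and CurrentAV also has a setter.
; The component is purely a data holder, with no active event logic.
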(event EventBeginPlay)

(event EventTick
  (params (DeltaSeconds :type Float%20%28single-precision%29)))

(fn FUInitializationAssignmentEnemy
  (params (CharacterAttributeBase :type ST%20Character%20Attribute%20Base%20Structure) (CharacterAttributeCombat :type ST%20Character%20Attribute%20Combat%20Structure) (Faction :type E_Faction%20Enum :default "NewEnumerator0") (ActionBarAvatar :type Texture%20Object%20Reference) (EnemyType :type E_EnemyType%20Enum :default "NewEnumerator0") (EnemyOccupation :type E_EnemyOccupation%20Enum :default "NewEnumerator0"))
  (Utilities|Struct|SetmembersinST_Attribute (Variables|Default|GetRuntimeAttribute) CharacterAttributeBase CharacterAttributeCombat Faction ActionBarAvatar EnemyType EnemyOccupation))

(fn FUGetActionBarAvatar
  (return (Utilities|Struct|BreakST_Attribute (Variables|Default|GetRuntimeAttribute))))

(fn FUInitializationAssignmentNOEnemy
  (params (CharacterAttributeBase :type ST%20Character%20Attribute%20Base%20Structure) (CharacterAttributeCombat :type ST%20Character%20Attribute%20Combat%20Structure) (Faction :type E_Faction%20Enum :default "NewEnumerator0") (ActionBarAvatar :type Texture%20Object%20Reference))
  (Utilities|Struct|SetmembersinST_Attribute (Variables|Default|GetRuntimeAttribute) CharacterAttributeBase CharacterAttributeCombat Faction ActionBarAvatar))

(fn FUGetSpeed
  (return (Utilities|Struct|BreakST_CharacterAttributeBase (.CharacterAttributeBase (Utilities|Struct|BreakST_Attribute (Variables|Default|GetRuntimeAttribute))))))

(fn FUGetCurrentAV
  (return (Utilities|Struct|BreakST_CharacterAttributeBase (.CharacterAttributeBase (Utilities|Struct|BreakST_Attribute (Variables|Default|GetRuntimeAttribute))))))

(fn FUSetCurrentAV
  (params (CurrentAV :type Float%20%28double-precision%29))
  (Utilities|Struct|SetmembersinST_CharacterAttributeBase (.CharacterAttributeBase (Utilities|Struct|BreakST_Attribute (Variables|Default|GetRuntimeAttribute))) CurrentAV))