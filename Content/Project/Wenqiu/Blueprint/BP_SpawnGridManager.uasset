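; BP_SpawnGridManager is an actor that lays out a flat grid of instanced static meshes.
; Its construction script calls FU_InitializationGridManager for a 10 by 10 grid, which uses nested loops to add instances to ISMGridManager, spaced by Interval.
; Instances are placed in world space starting one interval from the origin, so the layout ignores the actor's location.
; The event graph holds only disabled, empty default events.
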(event EventBeginPlay)

(event Collision|EventActorBeginOverlap
  (params (OtherActor :type Actor%20Object%20Reference)))

(event EventTick
  (params (DeltaSeconds :type Float%20%28single-precision%29)))

(fn ConstructionScript
  (CallFunction|FUInitializationGridManager 10 10))

(fn FUInitializationGridManager
  (params (GridX :type Integer) (GridY :type Integer))
  (bind _interval (Variables|Default|GetInterval))
  (for _index (range 1 GridX)
    (for _index_2 (range 1 GridY)
      (Components|InstancedStaticMesh|AddInstance (Variables|Default|GetISM_GridManager) (Math|Transform|MakeTransform (Math|Vector|MakeVector (Math|Conversions|ToFloat(Integer) (* _index _interval)) (Math|Conversions|ToFloat(Integer) (* _index_2 _interval)) 0.0) "0, 0, 0" "1.000000,1.000000,1.000000") true))))