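; Turn-based manager that orders all BP_CharacterBs actors on a speed-driven action-value (AV) timeline, where AV equals distance divided by Speed.
; Round initialization, not called here, seeds AVs, selection-sorts the queue and subtracts the leader's AV.
; A looping BeginPlay timer prints the queue, then after a delay resets the current unit's AV, reduces the others by the fastest unit's interval and re-sorts.
; An uncalled queue-jump helper swaps entries.
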(event Custom|自定义事件
  (Turn-based|FUStartTurn)
  (Utilities|FlowControl|Delay 2.0)
  (Turn-based|FUEndTurn))

(event EventBeginPlay
  (Utilities|Time|SetTimerbyEvent (delegate Custom|自定义事件) 3.0 true)
  (bind _returnvalue (Actor|GetActorOfClass "/Game/Project/Wenqiu/Character/BP_PlayerPawn.BP_PlayerPawn_C"))
  (Variables|Default|SetNewVar _returnvalue))

(event Collision|EventActorBeginOverlap
  (params (OtherActor :type Actor%20Object%20Reference)))

(event EventTick
  (params (DeltaSeconds :type Float%20%28single-precision%29)))

(fn ConstructionScript)

(fn FUInitializationAssignment
  (bind _outactors (Actor|GetAllActorsOfClass "/Game/Project/Wenqiu/Character/BP_CharacterBs.BP_CharacterBs_C"))
  (bind _output_get (Variables|Default|SetALLCharacter _outactors))
  (for _array_element _output_get
    (Utilities|Struct|SetmembersinBaseAttribute (Variables|/Script/FateOfTheKingdom.AttributeComponent|GetBaseAttribute (Variables|/Game/Project/Wenqiu/Character/BP_CharacterBs.BP_CharacterBs_C|GetCharacterAttributes _array_element)) (/ (Variables|Default|GetMaximumDistance) (Utilities|Struct|BreakBaseAttribute (Variables|/Script/FateOfTheKingdom.AttributeComponent|GetBaseAttribute (Variables|/Game/Project/Wenqiu/Character/BP_CharacterBs.BP_CharacterBs_C|GetCharacterAttributes _array_element)))))))

(fn FUEndTurn
  (Calculate|FUNextActionTurn))

(fn FUInitializeSorting
  (Variables|Default|SetQueueCache (Variables|Default|GetALLCharacter))
  ;[0.15 0.15 0.15 0.5] 移除无序数组，计算转换成有序数组
  (Utilities|Array|Clear (Variables|Default|GetALLCharacter))
  (LocalVariables|SetActionValueCache2 9999.0 :!label _label)
  (if (Utilities|Array|IsNotEmpty (Variables|Default|GetQueueCache))
    (for _array_element (Variables|Default|GetQueueCache)
      (if (< (Utilities|Struct|BreakBaseAttribute (Class|AttributeComponent|GetBaseAttribute (Variables|/Game/Project/Wenqiu/Character/BP_CharacterBs.BP_CharacterBs_C|GetCharacterAttributes _array_element))) (LocalVariables|GetActionValueCache2))
        (LocalVariables|SetActionValueCache2 (Utilities|Struct|BreakBaseAttribute (Class|AttributeComponent|GetBaseAttribute (Variables|/Game/Project/Wenqiu/Character/BP_CharacterBs.BP_CharacterBs_C|GetCharacterAttributes _array_element))))
        (Variables|Default|SetCurrentUnit _array_element)))
    (Utilities|Array|Add (Variables|Default|GetALLCharacter) (Variables|Default|GetCurrentUnit))
    (Utilities|Array|RemoveItem (Variables|Default|GetQueueCache) (Variables|Default|GetCurrentUnit))
    (goto _label)
    (else
      (Variables|Default|SetCurrentUnit (Utilities|Array|Get(acopy) (Variables|Default|GetALLCharacter)))
      (for _array_element_2 (Variables|Default|GetALLCharacter)
        (Utilities|Struct|SetmembersinBaseAttribute (Variables|/Script/FateOfTheKingdom.AttributeComponent|GetBaseAttribute (Variables|/Game/Project/Wenqiu/Character/BP_CharacterBs.BP_CharacterBs_C|GetCharacterAttributes _array_element_2)) (- (Utilities|Struct|BreakBaseAttribute (Variables|/Script/FateOfTheKingdom.AttributeComponent|GetBaseAttribute (Variables|/Game/Project/Wenqiu/Character/BP_CharacterBs.BP_CharacterBs_C|GetCharacterAttributes _array_element_2))) (Utilities|Struct|BreakBaseAttribute (Variables|/Script/FateOfTheKingdom.AttributeComponent|GetBaseAttribute (Variables|/Game/Project/Wenqiu/Character/BP_CharacterBs.BP_CharacterBs_C|GetCharacterAttributes (Variables|Default|GetCurrentUnit))))))))))

(fn FUStartTurn
  ;[0.15 0.15 0.15 0.5] 当前回合角色
  (CallFunction|FUCalculateCurrentTurnCharacter))

(fn FUNextActionTurn
  (for _array_element (Variables|Default|GetALLCharacter)
    (if (> (Utilities|Struct|BreakBaseAttribute (Variables|/Script/FateOfTheKingdom.AttributeComponent|GetBaseAttribute (Variables|/Game/Project/Wenqiu/Character/BP_CharacterBs.BP_CharacterBs_C|GetCharacterAttributes _array_element))) (LocalVariables|Getzuikuaispeed))
      (bind _output_get (LocalVariables|Setzuikuaispeed (Utilities|Struct|BreakBaseAttribute (Variables|/Script/FateOfTheKingdom.AttributeComponent|GetBaseAttribute (Variables|/Game/Project/Wenqiu/Character/BP_CharacterBs.BP_CharacterBs_C|GetCharacterAttributes _array_element)))))
      (LocalVariables|SetActionValueCache (/ (Variables|Default|GetMaximumDistance) _output_get))))
  (bind _output_get_2 (Variables|Default|SetQueueCache (Variables|Default|GetALLCharacter)))
  (Utilities|Array|RemoveItem _output_get_2 (Variables|Default|GetCurrentUnit))
  (Utilities|Struct|SetmembersinBaseAttribute (Variables|/Script/FateOfTheKingdom.AttributeComponent|GetBaseAttribute (Variables|/Game/Project/Wenqiu/Character/BP_CharacterBs.BP_CharacterBs_C|GetCharacterAttributes (Variables|Default|GetCurrentUnit))) (/ (Variables|Default|GetMaximumDistance) (Utilities|Struct|BreakBaseAttribute (Variables|/Script/FateOfTheKingdom.AttributeComponent|GetBaseAttribute (Variables|/Game/Project/Wenqiu/Character/BP_CharacterBs.BP_CharacterBs_C|GetCharacterAttributes (Variables|Default|GetCurrentUnit))))))
  (for _array_element_2 (Variables|Default|GetQueueCache)
    (Utilities|Struct|SetmembersinBaseAttribute (Variables|/Script/FateOfTheKingdom.AttributeComponent|GetBaseAttribute (Variables|/Game/Project/Wenqiu/Character/BP_CharacterBs.BP_CharacterBs_C|GetCharacterAttributes _array_element_2)) (Math|Float|Clamp(Float) (- (Utilities|Struct|BreakBaseAttribute (Variables|/Script/FateOfTheKingdom.AttributeComponent|GetBaseAttribute (Variables|/Game/Project/Wenqiu/Character/BP_CharacterBs.BP_CharacterBs_C|GetCharacterAttributes _array_element_2))) (LocalVariables|GetActionValueCache)) 0.0 1e+02))
    (if (> (LocalVariables|GetActionValueCache) (Math|Float|Clamp(Float) (- (Utilities|Struct|BreakBaseAttribute (Variables|/Script/FateOfTheKingdom.AttributeComponent|GetBaseAttribute (Variables|/Game/Project/Wenqiu/Character/BP_CharacterBs.BP_CharacterBs_C|GetCharacterAttributes _array_element_2))) (LocalVariables|GetActionValueCache)) 0.0 1e+02))
      (Variables|Default|SetCurrentUnit _array_element_2)))
  (Calculate|FUInitializeSorting))

(fn FUCuttingLineAnOrderQlyueue
  (bind _output_get (Variables|Default|SetQueueCache (Variables|Default|GetALLCharacter)))
  (Utilities|Array|RemoveItem _output_get (Variables|Default|GetCurrentUnit))
  (for (_array_element _array_index) _output_get
    (if (not (> (Utilities|Struct|BreakBaseAttribute (Variables|/Script/FateOfTheKingdom.AttributeComponent|GetBaseAttribute (Variables|/Game/Project/Wenqiu/Character/BP_CharacterBs.BP_CharacterBs_C|GetCharacterAttributes _array_element))) (Utilities|Struct|BreakBaseAttribute (Variables|/Script/FateOfTheKingdom.AttributeComponent|GetBaseAttribute (Variables|/Game/Project/Wenqiu/Character/BP_CharacterBs.BP_CharacterBs_C|GetCharacterAttributes (Variables|Default|GetCurrentUnit))))))
      (Utilities|Array|Swap (Variables|Default|GetALLCharacter) _array_index (Utilities|Array|FindItem (Variables|Default|GetALLCharacter) (Variables|Default|GetCurrentUnit)))))
  (Utilities|Array|Clear (Variables|Default|GetQueueCache))
  ;[0.15 0.15 0.15 0.5] 有序数组
  (for (_array_element_2 _array_index_2) (Variables|Default|GetALLCharacter)
    (Development|PrintString (Utilities|String|Append "序列：" (Utilities|String|ToString(Integer) _array_index_2) "     对象：" (Utilities|GetDisplayName _array_element_2) "  速度：" (Utilities|String|ToString(Float) (.Speed (Utilities|Struct|BreakBaseAttribute (Class|AttributeComponent|GetBaseAttribute (Variables|/Game/Project/Wenqiu/Character/BP_CharacterBs.BP_CharacterBs_C|GetCharacterAttributes _array_element_2))))) "     行动值：" (Utilities|String|ToString(Float) (.CurrentAV (Utilities|Struct|BreakBaseAttribute (Class|AttributeComponent|GetBaseAttribute (Variables|/Game/Project/Wenqiu/Character/BP_CharacterBs.BP_CharacterBs_C|GetCharacterAttributes _array_element_2)))))) true true "(R=0.023520,G=1.000000,B=0.905780,A=1.000000)")))

(fn FURoundInitialization
  ;[0.15 0.15 0.15 0.5] 给所有角色赋值行动条
  (Calculate|FUInitializationAssignment)
  ;[0.15 0.15 0.15 0.5] 无序数组转换为有序队列（方便UI ）
  (Calculate|FUInitializeSorting)
  (Turn-based|FUStartTurn))

(fn FUCalculateCurrentTurnCharacter
  ;[0.15 0.15 0.15 0.5] 有序数组
  (for (_array_element _array_index) (Variables|Default|GetALLCharacter)
    (Development|PrintString (Utilities|String|Append "序列：" (Utilities|String|ToString(Integer) _array_index) "     对象：" (Utilities|GetDisplayName _array_element) "  速度：" (Utilities|String|ToString(Float) (.Speed (Utilities|Struct|BreakBaseAttribute (Class|AttributeComponent|GetBaseAttribute (Variables|/Game/Project/Wenqiu/Character/BP_CharacterBs.BP_CharacterBs_C|GetCharacterAttributes _array_element))))) "     行动值：" (Utilities|String|ToString(Float) (.CurrentAV (Utilities|Struct|BreakBaseAttribute (Class|AttributeComponent|GetBaseAttribute (Variables|/Game/Project/Wenqiu/Character/BP_CharacterBs.BP_CharacterBs_C|GetCharacterAttributes _array_element)))))) true true "(R=0.023520,G=1.000000,B=0.905780,A=1.000000)")))