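; BPF_TurnActuator is a Blueprint function library that gives access to the turn-based manager and its combatant counts.
; A getter finds the BP_TurnbasedManager actor in the level with GetActorOfClass on each call, without caching it.
; Two queries use that getter to return the lengths of the manager's OutActors and OutEnemy arrays as character and enemy counts, along with a validity flag.
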(fn FUGetTurnManager
  (bind _returnvalue (Actor|GetActorOfClass 0 "/Game/Project/Wenqiu/Blueprint/BP_TurnbasedManager.BP_TurnbasedManager_C"))
  (return _returnvalue))

(fn FUReturnCurrentCharacters
  (bind _turnmanager (TurnManager|FUGetTurnManager))
  (Utilities|IsValid _turnmanager
    (:Is%20Valid
      (return (Utilities|Array|Length (Variables|/Game/Project/Wenqiu/Blueprint/BP_TurnbasedManager.BP_TurnbasedManager_C|GetOut%20Actors _turnmanager)) (Utilities|IsValid _turnmanager)))))

(fn FUReturnNumberEnemies
  (bind _turnmanager (TurnManager|FUGetTurnManager))
  (Utilities|IsValid _turnmanager
    (:Is%20Valid
      (return (Utilities|Array|Length (Variables|/Game/Project/Wenqiu/Blueprint/BP_TurnbasedManager.BP_TurnbasedManager_C|GetOut%20Enemy _turnmanager)) (Utilities|IsValid _turnmanager)))))