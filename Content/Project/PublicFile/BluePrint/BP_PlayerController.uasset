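; Player controller that sets up input, camera look and the player HUD for what appears to be a turn-based character game.
; On BeginPlay it adds the IMC_TestPlayer Enhanced Input mapping context, and IA_TestLook feeds yaw and pitch into the player pawn.
; Through a UI interface function it creates UMG_PlayerUI, stores it and initializes its queue with all characters.
; The character start-turn event is a stub that only prints a debug string.
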(event Input|EnhancedActionEvents|EnhancedInputActionIA_TestLook
  (params (ActionValue :type Vector%202D%20Structure) (ElapsedSeconds :type Float%20%28double-precision%29) (TriggeredSeconds :type Float%20%28double-precision%29) (InputAction :type Input%20Action%20Object%20Reference :default "/Game/Project/Wenqiu/Input/IA_TestLook.IA_TestLook"))
  (bind _returnvalue (Game|Player|GetPlayerPawn 0))
  (Pawn|Input|AddControllerYawInput _returnvalue (.x ActionValue))
  (Pawn|Input|AddControllerPitchInput _returnvalue (.y ActionValue)))

(event EventBeginPlay
  (Input|AddMappingContext (PlayerController|LocalPlayerSubsystems|GetEnhancedInputLocalPlayerSubsystem self) "/Game/Project/Wenqiu/Input/IMC_TestPlayer.IMC_TestPlayer" 0 "(bIgnoreAllPressedKeysUntilRelease=True,bForceImmediately=False,bNotifyUserSettings=False)"))

(event EventTick
  (params (DeltaSeconds :type Float%20%28single-precision%29)))

(event EventFUCharacterStartTurn
  (Development|PrintString "Hello"))

(fn ConstructionScript)

(fn FUUserWidgetInterface
  (params (AllCharacter :type Array%20of%20BP%20Character%20Bs%20Object%20References))
  (bind _returnvalue (UserInterface|CreateWidget "/Game/Project/Wenqiu/Widget/UMG_PlayerUI.UMG_PlayerUI_C"))
  (UserInterface|Viewport|AddtoViewport _returnvalue 0)
  (Variables|Default|SetUmgPlayer _returnvalue)
  (Default|FUInitializeQueue (Variables|Default|GetUmgPlayer) AllCharacter))