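; Game model Blueprint that bootstraps a turn-based grid battle when the level begins.
; It spawns the turn manager, grid manager and character manager, has the latter generate enemies and players on the grid, then the turn manager gathers all characters.
; It then initializes the player controller, passes the character list to its UI to build the ordered turn queue, and asks the turn manager to select the first actor.
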(event EventBeginPlay
  ;[0.15 0.15 0.15 0.5] 进入关卡初始化函数
  (CallFunction|FUInitialization)
  ;[0.15 0.15 0.15 0.5] 获取玩家控制器，BP_PlayerUI在玩家控制器中创建
  (bind _asbp_player_controller (Utilities|Casting|CastToBP_PlayerController (Game|GetPlayerController 0)))
  (Default|FUPlayerCharacterInitializationAssignment _asbp_player_controller)
  (Default|FUUserWidgetInterface _asbp_player_controller (Variables|/Game/Project/Wenqiu/Blueprint/BP_TurnbasedManager.BP_TurnbasedManager_C|GetALLCharacter (Variables|Default|GetTurnManagerReference)))
  ;[0.15 0.15 0.15 0.5] 查询当前最先行动的角色
  (Default|FUSelectNextTurn (Variables|Default|GetTurnManagerReference)))

(fn ConstructionScript)

(fn FUInitialization
  (Utilities|FlowControl|Sequence
    (:then_0
      ;[0.15 0.15 0.15 0.5] 生成回合制管理器
      (bind _returnvalue (Game|SpawnActorfromClass "/Game/Project/Wenqiu/Blueprint/BP_TurnbasedManager.BP_TurnbasedManager_C" (Math|Transform|MakeTransform "0, 0, 0" "0, 0, 0" "1.000000,1.000000,1.000000") "AlwaysSpawn" "MultiplyWithRoot" 0 0))
      (Variables|Default|SetTurnManagerReference _returnvalue))
    (:then_1
      ;[0.15 0.15 0.15 0.5] 生成战场格子
      (bind _returnvalue_2 (Game|SpawnActorfromClass "/Game/Project/Wenqiu/Blueprint/BP_SpawnGridManager.BP_SpawnGridManager_C" (Math|Transform|MakeTransform "0, 0, 0" "0, 0, 0" "1.000000,1.000000,1.000000") "AlwaysSpawn" "MultiplyWithRoot" 0 0))
      (Variables|Default|SetGridManager _returnvalue_2))
    (:then_2
      ;[0.15 0.15 0.15 0.5] 生成角色管理器，并执行生成敌人和玩家
      (bind _returnvalue_3 (Game|SpawnActorfromClass "/Game/Project/Wenqiu/Blueprint/BP_SpawnCharacterManager.BP_SpawnCharacterManager_C" (Math|Transform|MakeTransform "0, 0, 0" "0, 0, 0" "1.000000,1.000000,1.000000") "AlwaysSpawn" "MultiplyWithRoot" 0 0))
      (Default|FUInitializationGeneration _returnvalue_3 (Variables|Default|GetGridManager)))
    (:then_3
      ;[0.15 0.15 0.15 0.5] 回合制管理器初始化获取场上所有角色
      (Default|FUBattleBegins (Variables|Default|GetTurnManagerReference))
      (return))))