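; BP_AIControllerBase is an AI controller that takes turns for its controlled pawn in a turn-based system.
; On BeginPlay it finds and caches the BP_TurnbasedManager in the level.
; When its start-turn event fires, it prints the acting pawn's name, waits a fixed delay and tells the manager the turn is over, with no decision logic in between.
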(event EventBeginPlay
  (bind _returnvalue (Actor|GetActorOfClass "/Game/Project/Wenqiu/Blueprint/BP_TurnbasedManager.BP_TurnbasedManager_C"))
  (Variables|Default|SetBPTurnManager _returnvalue))

(event EventTick
  (params (DeltaSeconds :type Float%20%28single-precision%29)))

(event EventFUCharacterStartTurn
  (Development|PrintString (Utilities|String|Append "当前行动的角色：" (Utilities|GetDisplayName (Pawn|GetControlledPawn self))) true true "(R=1.000000,G=0.000000,B=0.354724,A=1.000000)")
  (Utilities|FlowControl|Delay 3.0)
  (Default|EventTurnOver (Variables|Default|GetBPTurnManager)))

(fn ConstructionScript)