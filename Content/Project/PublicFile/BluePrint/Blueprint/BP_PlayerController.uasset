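; Player controller for what appears to be a turn-based game with an action bar, handling test input, player UI and character stat setup.
; BeginPlay adds an Enhanced Input mapping context, and the look action drives the pawn's yaw and pitch.
; Separate functions create the player widget and initialize the BP_CheShi pawn's health, speed and avatar.
; The turn-start event prints a debug string and reveals a UI button.
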(event Custom|Event_ActionBarWidget)

(event Input|EnhancedActionEvents|EnhancedInputActionIA_TestLook
  (params (ActionValue :type Vector%202D%20Structure) (ElapsedSeconds :type Float%20%28double-precision%29) (TriggeredSeconds :type Float%20%28double-precision%29) (InputAction :type Input%20Action%20Object%20Reference :default "/Game/Project/Wenqiu/Input/IA_TestLook.IA_TestLook"))
  (bind _returnvalue (Game|Player|GetPlayerPawn 0))
  (Pawn|Input|AddControllerYawInput _returnvalue (.x ActionValue))
  (Pawn|Input|AddControllerPitchInput _returnvalue (.y ActionValue)))

(event EventBeginPlay
  (Input|AddMappingContext (PlayerController|LocalPlayerSubsystems|GetEnhancedInputLocalPlayerSubsystem self) "/Game/Project/Wenqiu/Input/IMC_TestPlayer.IMC_TestPlayer" 0 "(bIgnoreAllPressedKeysUntilRelease=True,bForceImmediately=False,bNotifyUserSettings=False)"))

(event EventFUCharacterStartTurn
  (Development|PrintString "Hello")
  (Widget|SetVisibility (Variables|/Game/Project/Wenqiu/Widget/UMG_PlayerUI.UMG_PlayerUI_C|GetButton_0 (Variables|Default|GetUmgPlayer)) "Visible"))

(fn ConstructionScript)

(fn FUUserWidgetInterface
  (bind _returnvalue (UserInterface|CreateWidget "/Game/Project/Wenqiu/Widget/UMG_PlayerUI.UMG_PlayerUI_C"))
  (UserInterface|Viewport|AddtoViewport _returnvalue 0)
  (Variables|Default|SetUmgPlayer _returnvalue))

(fn FUPlayerCharacterInitializationAssignment
  (bind _asbp_che_shi (Utilities|Casting|CastToBP_CheShi (Game|Player|GetPlayerPawn 0)))
  (Default|FUInitializationAssignmentNOEnemy :self (Variables|/Game/Project/Wenqiu/Character/BP_CharacterBs.BP_CharacterBs_C|GetBP_CharacterAttribute _asbp_che_shi) :CharacterAttributeBase (Utilities|Struct|MakeST_CharacterAttributeBase 1e+02 1e+02 0 0 8e+01 0.0 0.0 0) :ActionBarAvatar "/Game/Project/Shadow/Assets/Image/ailisi.ailisi"))