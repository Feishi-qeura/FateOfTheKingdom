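; BP_CheShi is a character Blueprint, apparently for testing, that extends a parent class with player input and a turn-finish override.
; The IA_Move input action passes its value to CharacterState for WASD movement, and a hard-wired NumPad 1 key asks CharacterState to attempt an attack on the look-at target.
; FU_FinishTurn prints a placeholder debug string before calling the parent implementation.
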(event Input|EnhancedActionEvents|EnhancedInputActionIA_Move
  (params (ActionValue :type Vector%202D%20Structure) (ElapsedSeconds :type Float%20%28double-precision%29) (TriggeredSeconds :type Float%20%28double-precision%29) (InputAction :type Input%20Action%20Object%20Reference :default "/Game/Project/zhiYin/Input/IA_Move.IA_Move"))
  (Class|CharacterStateComponent|MoveInputWASD (Variables|Default|GetCharacterState) ActionValue))

(event EventBeginPlay
  (|CallParentFunction))

(event Collision|EventActorBeginOverlap
  (params (OtherActor :type Actor%20Object%20Reference))
  (|CallParentFunction OtherActor) ; 此节点被禁用，将不会被调用。\n从引脚连出引线来编译功能。
)

(event EventTick
  (params (DeltaSeconds :type Float%20%28single-precision%29))
  (|CallParentFunction DeltaSeconds) ; 此节点被禁用，将不会被调用。\n从引脚连出引线来编译功能。
)

(event Input|KeyboardEvents|NumPadOne
  (params (Key :type Key%20Structure :default "None"))
  (:Pressed
    (Class|CharacterStateComponent|TryAttackLookatTarget (Variables|Default|GetCharacterState) 2.0)))

(fn ConstructionScript
  (|CallParentFunction))

(fn FUFinishTurn
  (Development|PrintString "asdawefrvsdfc")
  (|CallParentFunction))

(fn NewEventDispatcherEvent)